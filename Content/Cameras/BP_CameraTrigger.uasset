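; BP_CameraTrigger is a trigger volume that activates and deactivates a camera as the player moves through it.
; When a BP_CPlayer enters the Box, it calls OnBeginOverlap on the Camera, and when the player leaves it calls OnFinish.
; If no valid Camera is set, it falls back to the first BP_CCameraActor found in the level.
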(event `self.Box.OnComponentBeginOverlap`
  (params (OverlappedComponent :type "PrimitiveComponent Object Reference") (OtherActor :type "Actor Object Reference") (OtherComp :type "PrimitiveComponent Object Reference") (OtherBodyIndex :type Integer) (bFromSweep :type Boolean) (SweepResult :type "HitResult Structure (by ref)"))
  (cast `/Game/Player/BP_CPlayer` OtherActor)
  (`self.Camera`
    (:`then`
      _)
    (:`else`
      (bind _outactors (`GameplayStatics.GetAllActorsOfClass` "/Game/Cameras/BP_CCameraActor.BP_CCameraActor_C"))
      (bind _output_get (set `self.Camera` (`|GetArrayItem` _outactors)))))
  (`CCameraActor.OnBeginOverlap` _output_get))

(event `self.Box.OnComponentEndOverlap`
  (params (OverlappedComponent :type "PrimitiveComponent Object Reference") (OtherActor :type "Actor Object Reference") (OtherComp :type "PrimitiveComponent Object Reference") (OtherBodyIndex :type Integer))
  (cast `/Game/Player/BP_CPlayer` OtherActor)
  (`self.Camera`
    (:`then`
      _)
    (:`else`
      (bind _outactors (`GameplayStatics.GetAllActorsOfClass` "/Game/Cameras/BP_CCameraActor.BP_CCameraActor_C"))
      (bind _output_get (set `self.Camera` (`|GetArrayItem` _outactors)))))
  (`CCameraActor.OnFinish` _output_get))

(fn `UserConstructionScript`)